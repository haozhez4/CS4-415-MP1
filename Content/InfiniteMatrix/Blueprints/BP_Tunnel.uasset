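; BP_Tunnel is a tunnel segment with a spinning holed wall for an endless dodging game, with a function to randomize the wall's mesh and roll.
; Wall overlap drains BP_Player's blood, flags a hit, and can trigger death and restart display.
; The trigger zone spawns the next tunnel, destroys itself and linked pickup or enemy, and scores unhit passes.
; Each segment's BeginPlay also adds a new blood bar widget to the viewport.
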(event `self.ReceiveBeginPlay`
  (bind _returnvalue (`|CreateWidget` "/Game/InfiniteMatrix/UI/UI_Blood_Bar.UI_Blood_Bar_C"))
  (`UserWidget.AddToViewport` _returnvalue 0))

(event `self.ReceiveTick`
  (params (DeltaSeconds :type "Float (single-precision)"))
  (`SceneComponent.K2_AddLocalRotation` (`self.WallMesh`) (`KismetMathLibrary.MakeRotator` (* DeltaSeconds (`self.RotateSpeed`))) false false))

(event `self.TriggerZone.OnComponentBeginOverlap`
  (params (OverlappedComponent :type "PrimitiveComponent Object Reference") (OtherActor :type "Actor Object Reference") (OtherComp :type "PrimitiveComponent Object Reference") (OtherBodyIndex :type Integer) (bFromSweep :type Boolean) (SweepResult :type "HitResult Structure (by ref)"))
  (bind _destroyenemy (`self.DestroyEnemy`))
  (bind _destroyhealthpack (`self.DestroyHealthPack`))
  (bind _asbp_player (cast `/Game/InfiniteMatrix/Blueprints/BP_Player` OtherActor))
  (`|ExecutionSequence`
    (:`then_0`
      (bind _asbp_player_2 (cast `/Game/InfiniteMatrix/Blueprints/BP_Player` OtherActor))
      (`/Game/InfiniteMatrix/Blueprints/BP_TunnelSpawner.SpawnTunnelAtSpawnPoint` (`self.TunnelSpawner`))
      (`|ExecutionSequence`
        (:`then_0`
          (`/Engine/EditorBlueprintResources/StandardMacros.IsValid` _destroyenemy
            (:`Is Valid`
              (`self.K2_DestroyActor` _destroyenemy))
            (:`Is Not Valid`
              (`self.K2_DestroyActor` :!label _label))))
        (:`then_1`
          (`/Engine/EditorBlueprintResources/StandardMacros.IsValid` _destroyhealthpack
            (:`Is Valid`
              (`self.K2_DestroyActor` _destroyhealthpack)
              (goto _label))
            (:`Is Not Valid`
              (goto _label))))))
    (:`then_1`
      (if (`/Game/InfiniteMatrix/Blueprints/BP_Player.Hit` _asbp_player)
        (set `/Game/InfiniteMatrix/Blueprints/BP_Player.Hit` false _asbp_player_2)
        (else
          (bind _asbp_player_3 (cast `/Game/InfiniteMatrix/Blueprints/BP_Player` OtherActor))
          (bind _output_get (set `self.As BP Player` _asbp_player_3))
          (set `/Game/InfiniteMatrix/Blueprints/BP_Player.Score` (+ (`/Game/InfiniteMatrix/Blueprints/BP_Player.Score` (`self.As BP Player`)) 1) _output_get))))))

(event `self.WallMesh.OnComponentBeginOverlap`
  (params (OverlappedComponent :type "PrimitiveComponent Object Reference") (OtherActor :type "Actor Object Reference") (OtherComp :type "PrimitiveComponent Object Reference") (OtherBodyIndex :type Integer) (bFromSweep :type Boolean) (SweepResult :type "HitResult Structure (by ref)"))
  (bind _returnvalue (- (`/Game/InfiniteMatrix/Blueprints/BP_Player.Blood_Now` (`self.As BP Player`)) 10))
  (bind _asbp_player (cast `/Game/InfiniteMatrix/Blueprints/BP_Player` OtherActor))
  (`|ExecutionSequence`
    (:`then_0`
      (bind _asbp_player_2 (cast `/Game/InfiniteMatrix/Blueprints/BP_Player` OtherActor))
      (bind _output_get (set `self.As BP Player` _asbp_player_2))
      (if (`KismetMathLibrary.Conv_IntToBool` _returnvalue)
        (set `/Game/InfiniteMatrix/Blueprints/BP_Player.Blood_Now` _returnvalue _output_get)
        (else
          (set `/Game/InfiniteMatrix/Blueprints/BP_Player.IsDead` true _asbp_player_2)
          (set `/Game/InfiniteMatrix/Blueprints/BP_Player.Blood_Now` 0 _asbp_player_2)
          (`/Game/InfiniteMatrix/Blueprints/BP_Player.DisplayRestart` _asbp_player_2))))
    (:`then_1`
      (set `/Game/InfiniteMatrix/Blueprints/BP_Player.Hit` true _asbp_player))))

(fn `RandomizeWall`
  (`StaticMeshComponent.SetStaticMesh` (`self.WallMesh`) (select `int` (`KismetMathLibrary.RandomIntegerInRange` 0 3) :`0` "/Game/InfiniteMatrix/Meshes/SM_Hole_01.SM_Hole_01" :`1` "/Game/InfiniteMatrix/Meshes/SM_Hole_02.SM_Hole_02" :`2` "/Game/InfiniteMatrix/Meshes/SM_Hole_03.SM_Hole_03" :`3` "/Game/InfiniteMatrix/Meshes/SM_Hole_04.SM_Hole_04" :!type "StaticMesh Object Reference"))
  (`SceneComponent.K2_AddLocalRotation` (`self.WallMesh`) (`KismetMathLibrary.MakeRotator` (`KismetMathLibrary.RandomFloatInRange` 0.0 360.0)) false false))

(fn `UserConstructionScript`)