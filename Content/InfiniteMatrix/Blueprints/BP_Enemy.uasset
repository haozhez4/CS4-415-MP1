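; BP_Enemy is a spinning rock hazard that damages the player on contact and can be shot for score.
; Tick rotates the Rock component on all axes by RotateSpeed, scaled by delta time.
; Rock overlap with BP_Player subtracts health, or triggers death and the restart display when the result would be exactly zero, then destroys the rock.
; Overlap with BP_Bullet destroys the rock and increments the player's Score.
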(event `self.ReceiveTick`
  (params (DeltaSeconds :type "Float (single-precision)"))
  (bind _returnvalue (* DeltaSeconds (`self.RotateSpeed`)))
  (`SceneComponent.K2_AddLocalRotation` (`self.Rock`) (`KismetMathLibrary.MakeRotator` _returnvalue _returnvalue _returnvalue) false false))

(event `self.Rock.OnComponentBeginOverlap`
  (params (OverlappedComponent :type "PrimitiveComponent Object Reference") (OtherActor :type "Actor Object Reference") (OtherComp :type "PrimitiveComponent Object Reference") (OtherBodyIndex :type Integer) (bFromSweep :type Boolean) (SweepResult :type "HitResult Structure (by ref)"))
  (`|ExecutionSequence`
    (:`then_0`
      (bind _asbp_player (cast `/Game/InfiniteMatrix/Blueprints/BP_Player` OtherActor))
      (bind _returnvalue (- (`/Game/InfiniteMatrix/Blueprints/BP_Player.Blood_Now` _asbp_player) 10))
      (if (`KismetMathLibrary.Conv_IntToBool` _returnvalue)
        (set `/Game/InfiniteMatrix/Blueprints/BP_Player.Blood_Now` _returnvalue _asbp_player)
        (else
          (set `/Game/InfiniteMatrix/Blueprints/BP_Player.IsDead` true _asbp_player)
          (set `/Game/InfiniteMatrix/Blueprints/BP_Player.Blood_Now` 0 _asbp_player)
          (`/Game/InfiniteMatrix/Blueprints/BP_Player.DisplayRestart` _asbp_player)))
      (`self.K2_DestroyActor`))
    (:`then_1`
      (cast `/Game/InfiniteMatrix/Blueprints/BP_Bullet` OtherActor)
      (`self.K2_DestroyActor`)
      (bind _asbp_player_2 (cast `/Game/InfiniteMatrix/Blueprints/BP_Player` (`GameplayStatics.GetPlayerPawn` 0)))
      (set `/Game/InfiniteMatrix/Blueprints/BP_Player.Score` (+ (`/Game/InfiniteMatrix/Blueprints/BP_Player.Score` _asbp_player_2) 1) _asbp_player_2))))

(fn `UserConstructionScript`)