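; BP_TunnelSpawner builds the chain of tunnel segments the player travels through, populated with random enemies and health packs.
; On BeginPlay it clears existing tunnels, then spawns a short starting run from the player pawn's location.
; Each new segment attaches at the newest tunnel's SpawnPoint, randomizes its wall and receives a spawner reference for callbacks.
; Coin flips decide each pickup and enemy spawn, which the tunnel stores, apparently for cleanup.
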(event `self.ReceiveBeginPlay`
  (`self.Spawn Initial Tunnels`))

(fn `Spawn Initial Tunnels`
  (`|ExecutionSequence`
    (:`then_0`
      (`GameplayStatics.GetAllActorsOfClass` "/Game/InfiniteMatrix/Blueprints/BP_Tunnel.BP_Tunnel_C")
      (for _array_element _
        (`self.K2_DestroyActor` _array_element)))
    (:`then_1`
      (for _ (range 3)
        (`/Engine/EditorBlueprintResources/StandardMacros.IsValid` (`self.NewestTunnel`)
          (:`Is Valid`
            (`self.SpawnTunnelAtSpawnPoint`))
          (:`Is Not Valid`
            (`self.SpawnTunnel` (`self.K2_GetActorLocation` (`GameplayStatics.GetPlayerPawn` 0)))))))))

(fn `SpawnTunnel`
  (params (SpawnLocation :type "Vector Structure"))
  (locals (NewLocalVar :type "/Game/InfiniteMatrix/Blueprints/BP_TunnelSpawner Object Reference"))
  (bind _returnvalue (`|SpawnActorFromClass` "/Game/InfiniteMatrix/Blueprints/BP_Tunnel.BP_Tunnel_C" (`KismetMathLibrary.MakeTransform` (`KismetMathLibrary.MakeVector` SpawnLocation_X SpawnLocation_Y SpawnLocation_Z)) "Undefined" "MultiplyWithRoot" null null))
  (bind _output_get (set `self.NewestTunnel` _returnvalue))
  (set `/Game/InfiniteMatrix/Blueprints/BP_Tunnel.TunnelSpawner` self _output_get)
  (`/Game/InfiniteMatrix/Blueprints/BP_Tunnel.RandomizeWall` _output_get)
  (`|ExecutionSequence`
    (:`then_0`
      (if (`KismetMathLibrary.RandomBool`)
        (bind _returnvalue_2 (`|SpawnActorFromClass` "/Game/InfiniteMatrix/Blueprints/BP_Enemy.BP_Enemy_C" (`KismetMathLibrary.MakeTransform` (`KismetMathLibrary.MakeVector` (+ (`KismetMathLibrary.RandomFloatInRange` 200.0 2400.0) SpawnLocation_X) (+ (`KismetMathLibrary.RandomFloatInRange` -200.0 200.0) SpawnLocation_Y) (+ (`KismetMathLibrary.RandomFloatInRange` -200.0 200.0) SpawnLocation_Z)) (`KismetMathLibrary.MakeRotator` (`KismetMathLibrary.RandomFloatInRange` 0.0 360.0))) "Undefined" "MultiplyWithRoot" null null))
        (set `/Game/InfiniteMatrix/Blueprints/BP_Tunnel.DestroyEnemy` _returnvalue_2 _returnvalue)))
    (:`then_1`
      (if (`KismetMathLibrary.RandomBool`)
        (bind _returnvalue_3 (`|SpawnActorFromClass` "/Game/InfiniteMatrix/Blueprints/BP_Health_Pack.BP_Health_Pack_C" (`KismetMathLibrary.MakeTransform` (`KismetMathLibrary.MakeVector` (+ SpawnLocation_X (`KismetMathLibrary.RandomFloatInRange` 200.0 2400.0)) (+ SpawnLocation_Y (`KismetMathLibrary.RandomFloatInRange` -200.0 200.0)) (+ SpawnLocation_Z (`KismetMathLibrary.RandomFloatInRange` -200.0 200.0))) (`KismetMathLibrary.MakeRotator` (`KismetMathLibrary.RandomFloatInRange` 0.0 360.0))) "Undefined" "MultiplyWithRoot" null null))
        (set `/Game/InfiniteMatrix/Blueprints/BP_Tunnel.DestroyHealthPack` _returnvalue_3 _returnvalue)))))

(fn `SpawnTunnelAtSpawnPoint`
  (`self.SpawnTunnel` (`SceneComponent.K2_GetComponentLocation` (`/Game/InfiniteMatrix/Blueprints/BP_Tunnel.SpawnPoint` (`self.NewestTunnel`)))))

(fn `UserConstructionScript`)