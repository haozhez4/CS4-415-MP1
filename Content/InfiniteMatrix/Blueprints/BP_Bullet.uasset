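; BP_Bullet is a projectile actor that flies along world X and speeds up as the player's score rises.
; Each Tick it casts the player pawn to BP_Player, picks a speed bonus from Score thresholds, and adds it to ForwardSpeed for a swept, delta-time-scaled world offset.
; Any begin overlap on its Bullet component destroys the actor, with no other hit handling.
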(event `self.Bullet.OnComponentBeginOverlap`
  (params (OverlappedComponent :type "PrimitiveComponent Object Reference") (OtherActor :type "Actor Object Reference") (OtherComp :type "PrimitiveComponent Object Reference") (OtherBodyIndex :type Integer) (bFromSweep :type Boolean) (SweepResult :type "HitResult Structure (by ref)"))
  (`self.K2_DestroyActor`))

(event `self.ReceiveTick`
  (params (DeltaSeconds :type "Float (single-precision)"))
  (bind _asbp_player (cast `/Game/InfiniteMatrix/Blueprints/BP_Player` (`GameplayStatics.GetPlayerPawn` 0)))
  (bind _score (`/Game/InfiniteMatrix/Blueprints/BP_Player.Score` _asbp_player))
  (if (>= _score 40)
    (if (>= _score 60)
      (if (>= _score 80)
        (`self.K2_AddActorWorldOffset` (`KismetMathLibrary.MakeVector` (* DeltaSeconds (+ 1500.0 (`self.ForwardSpeed`)))) true)
        (else
          (`self.K2_AddActorWorldOffset` (`KismetMathLibrary.MakeVector` (* DeltaSeconds (+ 1000.0 (`self.ForwardSpeed`)))) true)))
      (else
        (`self.K2_AddActorWorldOffset` (`KismetMathLibrary.MakeVector` (* DeltaSeconds (+ 500.0 (`self.ForwardSpeed`)))) true)))
    (else
      (`self.K2_AddActorWorldOffset` (`KismetMathLibrary.MakeVector` (* DeltaSeconds (`self.ForwardSpeed`))) true))))

(fn `UserConstructionScript`)